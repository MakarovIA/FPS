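; Child Blueprint of a soldier character that slaves a separate Head component to the body Mesh through master pose in the construction script.
; BeginPlay and Tick defer to the parent; BeginPlay also caches the starting location and casts the controller to AIController, with nothing following the cast.
; Disconnected leftover nodes cover a debug movement trail, head bone hiding, a controller ID lookup and head owner visibility.
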(event `self.ReceiveBeginPlay`
  (`parent.ReceiveBeginPlay`)
  (set `self.Previous Location` (`SceneComponent.K2_GetComponentLocation` (`self.Scene`)))
  (cast `AIController` (`self.GetController`)))

(event `self.ReceiveTick`
  (params (DeltaSeconds :type "Float (single-precision)"))
  (`parent.ReceiveTick` DeltaSeconds))

(fn `UserConstructionScript`
  (`parent.UserConstructionScript`)
  (`SkinnedMeshComponent.SetLeaderPoseComponent` (`self.Head`) (`self.Mesh`)))