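; Hitscan rifle Blueprint for a bot-owned weapon that handles firing effects and damage.
; OnFire repeatedly calls GetHitData with the aim rotation to gather hit details, then plays the shot sound and draws a debug tracer.
; Blocking hits spawn an explosion, and fire attached to any hit actor, using the hit bone on Bots.
; Only Bots take the randomized point damage, credited to the owning bot's controller.
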(event `self.OnFire`
  (bind _outhit (`self.GetHitData` (`self.GetAimRotation`)))
  (bind _returnvalue (`KismetMathLibrary.Conv_VectorToTransform` (`self.HitLocation`)))
  (bind (_bblockinghit _binitialoverlap _time _location _impactpoint _normal _impactnormal _physmat _hitactor _hitcomponent _hitbonename _hititem _tracestart _traceend) (`GameplayStatics.BreakHitResult` _outhit))
  ;[1 1 1] Gather Data
  (`|ExecutionSequence`
    (:`then_0`
      (set `self.HitLocation` _location))
    (:`then_1`
      (set `self.HitActor` _hitactor))
    (:`then_2`
      (bind _output_get (set `self.TraceStart` _tracestart)))
    (:`then_3`
      (set `self.Hit` _outhit))
    (:`then_4`
      (set `self.HitBone` _hitbonename)
      ;[1 1 1] Effects
      (`GameplayStatics.PlaySoundAtLocation` null "/Game/Weapons/Rifle/Sounds/AssaultRifle_Shot.AssaultRifle_Shot" _output_get)
      (if _bblockinghit
        (`KismetSystemLibrary.DrawDebugLine` null (`self.TraceStart`) (`self.HitLocation`) (struct :`R` 1.0 :`A` 1.0) 0.0)
        (`|SpawnActorFromClass` "/Game/StarterContent/Blueprints/Blueprint_Effect_Explosion.Blueprint_Effect_Explosion_C" _returnvalue "AlwaysSpawn" "OverrideRootScale")
        (`/Engine/EditorBlueprintResources/StandardMacros.IsValid` (`self.HitActor`)
          (:`Is Valid`
            (bind _returnvalue_2 (`|SpawnActorFromClass` "/Game/StarterContent/Blueprints/Blueprint_Effect_Fire.Blueprint_Effect_Fire_C" _returnvalue "AdjustIfPossibleButDontSpawnIfColliding" "OverrideRootScale"))
            (bind _asbot (cast `Bot` (`self.HitActor`))
              (:`then`
                (`self.K2_AttachRootComponentTo` _returnvalue_2 (`Character.Mesh` _asbot) (`self.HitBone`) "KeepWorldPosition" true))
              (:`CastFailed`
                (`self.K2_AttachRootComponentToActor` _returnvalue_2 (`self.HitActor`) "None" "KeepWorldPosition" true)))
            ;[1 1 1] Damage
            (bind _asbot_2 (cast `Bot` (`self.HitActor`)))
            (`GameplayStatics.ApplyPointDamage` _asbot_2 (`KismetMathLibrary.RandomFloatInRange` 7.0 11.0) (- (`self.HitLocation`) (`self.TraceStart`)) (`self.Hit`) (`Pawn.GetController` (`self.OwningBot`)) self)))
        (else
          (`KismetSystemLibrary.DrawDebugLine` null _output_get _traceend (struct :`R` 1.0 :`A` 1.0)))))))

(fn `UserConstructionScript`)